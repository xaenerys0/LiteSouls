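; Hero character Blueprint that routes attack input into an ability actor component.
; The component initializes one second after BeginPlay, and the light attack input asks it to activate an ability, while heavy attack only prints a debug string.
; Helper functions expose the light attack montage with its play length and a self reference, and an event sets max walk speed.
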(event `self.ReceiveBeginPlay`
  (`KismetSystemLibrary.Delay` 1.0)
  (`/Game/BP_AbilityActorComponent.Initialize` (`self.BP_AbilityActorComponent`)))

(event `/Game/INT_HeroChar.SetPlayerSpeed`
  (params (Speed :type "Float (single-precision)"))
  (set `CharacterMovementComponent.MaxWalkSpeed` Speed (`self.CharacterMovement`)))

(event `InputAction|LightAttack`
  (params (Key :type "Key Structure"))
  (:`Pressed`
    (`/Game/BP_AbilityActorComponent.TryToActivateAbility` (`self.BP_AbilityActorComponent`) (`self.Abilities`))))

(event `InputAction|HeavyAttack`
  (params (Key :type "Key Structure"))
  (:`Pressed`
    (`KismetSystemLibrary.PrintString` "Heavy attack")))

(fn `GetMeleeAttackInfo`
  (returns (Montage :type "AnimMontage Object Reference") (Length :type "Float (double-precision)"))
  (locals (L_Montage :type "AnimMontage Object Reference"))
  (bind _output_get (set `local.L_Montage` "/Game/LightAttack_Montage.LightAttack_Montage"))
  (bind _returnvalue (`AnimSequenceBase.GetPlayLength` _output_get))
  (return _output_get _returnvalue))

(fn `HeroCharRef`
  (returns (HeroChar :type "/Game/BP_HeroChar Object Reference"))
  (return self))

(fn `UserConstructionScript`)