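; Actor component that runs player ability activation, currently supporting a melee light attack.
; On Initialize it caches the owning hero through an interface message.
; TryToActivateAbility switches on the selected ability and, for Light Attack, plays the montage from the hero's melee attack info on its mesh.
; An IsAttacking flag blocks repeat attacks until the montage completes, with debug prints marking each step.
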(event `Initialize`
  (`KismetSystemLibrary.PrintString` "Ability Component Initialized")
  (bind _herochar (message `/Game/INT_HeroChar.HeroCharRef` (`self.GetOwner`)))
  (set `self.Player` _herochar))

(event `TryToActivateAbility`
  (params (SelectedAbility :type "ESelectedAbility Enum" :default "None"))
  (bind _player (`self.Player`))
  (`/Engine/EditorBlueprintResources/StandardMacros.IsValid` (`self.Player`)
    (:`Is Valid`
      (switch `ESelectedAbility` SelectedAbility
        (:`LightAttack`
          (if (not (`self.IsAttacking`))
            (`KismetSystemLibrary.PrintString` "Light attacking")
            (set `self.IsAttacking` true)
            (bind _montage (message `/Game/INT_HeroChar.GetMeleeAttackInfo` _player))
            (`|PlayMontage` (`Character.Mesh` _player) _montage
              (:`OnCompleted`
                (set `self.IsAttacking` false)
                (`KismetSystemLibrary.PrintString` "Light attack done")))
            (else
              (`KismetSystemLibrary.PrintString` "Already attacking"))))))))